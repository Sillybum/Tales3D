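; BP_Human is a human character Blueprint that drives a combo basic attack from target-based attack input.
; Its Combat object validates each attack, tracks the combo count and queues follow-up input.
; The first hit plays AM_BasicAttack from its opening section, and consumed follow-up inputs jump the montage to the current combo section.
; A montage-ended delegate bound on BeginPlay ends the attack, with debug prints left in.
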(event `self.BP_OnBasicAttackInput`
  (params (Target :type "Enemy Object Reference"))
  (bind _combat (`self.Combat`))
  (bind _combat_2 (`self.Combat`))
  (bind _returnvalue (`SkeletalMeshComponent.GetAnimInstance` (`self.Mesh`)))
  (`/Engine/EditorBlueprintResources/StandardMacros.IsValid` Target
    (:`Is Valid`
      (`/Engine/EditorBlueprintResources/StandardMacros.IsValid` _combat_2
        (:`Is Valid`
          (if (`CombatComponent.CanStartBasicAttack` _combat_2 Target)
            (if (== (`CombatComponent.GetCurrentCombo` _combat_2) 0)
              (`CombatComponent.BeginBasicAttack` _combat Target 5)
              (`AnimInstance.Montage_Play` _returnvalue "/Game/_Core/Char/Shared/Human/Anim/Montage/AM_BasicAttack.AM_BasicAttack" 1.0 "MontageLength" 0.0 true)
              (`AnimInstance.Montage_JumpToSection` _returnvalue "A1" "/Game/_Core/Char/Shared/Human/Anim/Montage/AM_BasicAttack.AM_BasicAttack")
              (else
                (`CombatComponent.QueueBasicInput` _combat)
                (bind _returnvalue_2 (`CombatComponent.TryConsumeInputAndAdvance` _combat))
                (if _returnvalue_2
                  (`AnimInstance.Montage_JumpToSection` (`SkeletalMeshComponent.GetAnimInstance` (`self.Mesh`)) (`CombatComponent.GetCurrentComboSection` (`self.Combat`)) "/Game/_Core/Char/Shared/Human/Anim/Montage/AM_BasicAttack.AM_BasicAttack")
                  (`KismetSystemLibrary.PrintString` "A2"))))))))))

(event `self.ReceiveBeginPlay`
  (`parent.ReceiveBeginPlay`)
  (add `AnimInstance.OnMontageEnded` (`SkeletalMeshComponent.GetAnimInstance` (`self.Mesh`)) (delegate `OnMontageEnded_Event`)))

(event `OnMontageEnded_Event`
  (params (Montage :type "AnimMontage Object Reference") (bInterrupted :type Boolean))
  (if (== Montage "/Game/_Core/Char/Shared/Human/Anim/Montage/AM_BasicAttack.AM_BasicAttack")
    (`CombatComponent.EndBasicAttack` (`self.Combat`))
    (`KismetSystemLibrary.PrintString` "montage ended")))

(fn `UserConstructionScript`)