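; Weapon afterimage effect actor, meant to show a fading ghost of a weapon and then destroy itself.
; On init it assigns the weapon's static mesh component itself to SMWeaponGhost, then applies a tinted M_AfterImage dynamic material to slot 0.
; TL_Fade updates opacity with a Lerp whose alpha is fixed at zero, so opacity holds at StartOpacity until the timeline finishes and the actor is destroyed.
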(event `Event_InitFromWeaponActor`
  (params (WeaponActor :type "Actor Object Reference"))
  (bind _mid (`self.MID`))
  (`/Engine/EditorBlueprintResources/StandardMacros.IsValid` WeaponActor
    (:`Is Valid`
      (bind _output_get (set `self.SrcSM` (`self.GetComponentByClass` WeaponActor "/Script/Engine.StaticMeshComponent")))
      (`/Engine/EditorBlueprintResources/StandardMacros.IsValid` _output_get
        (:`Is Valid`
          (bind _output_get_2 (set `self.SM_WeaponGhost` _output_get))
          (`SceneComponent.K2_SetWorldTransform` _output_get_2 (`SceneComponent.K2_GetComponentToWorld` _output_get) false false)
          (bind _returnvalue (`KismetMaterialLibrary.CreateDynamicMaterialInstance` "/Game/_Core/FX/M_AfterImage.M_AfterImage"))
          (bind _output_get_3 (set `self.MID` _returnvalue))
          (`MaterialInstanceDynamic.SetVectorParameterValue` _output_get_3 "Tint" (`self.Tint`))
          (`MaterialInstanceDynamic.SetScalarParameterValue` _output_get_3 "Opacity" (`self.StartOpacity`))
          (`PrimitiveComponent.SetMaterial` (`self.SM_WeaponGhost`) 0 (`self.MID`))
          (`Timeline|TL_Fade`
            (:`Update`
              (`/Engine/EditorBlueprintResources/StandardMacros.IsValid` _mid
                (:`Is Valid`
                  (`MaterialInstanceDynamic.SetScalarParameterValue` _mid "Opacity" (`KismetMathLibrary.Lerp` (`self.StartOpacity`))))))
            (:`Finished`
              (`self.K2_DestroyActor`))))))))

(fn `UserConstructionScript`)