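; BP_AfterImage is a short-lived ghost actor that leaves a tinted, fading afterimage of a skeletal mesh.
; InitFromMesh freezes the source's pose onto the poseable mesh PMGhost and applies a dynamic M_AfterImage material to slot 0 only.
; The TL_Fade timeline lerps opacity from start to end value, then the actor destroys itself.
; The Transform input is unused, so placement is not handled here.
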(event `Event_InitFromMesh`
  (params (SourceMesh :type "SkeletalMeshComponent Object Reference") (Transform :type "Transform Structure"))
  (bind _mid (`self.MID`))
  (bind _mid_2 (`self.MID`))
  (`PoseableMeshComponent.CopyPoseFromSkeletalComponent` (`self.PM_Ghost`) SourceMesh)
  ; Sets Material
  (bind _returnvalue (`KismetMaterialLibrary.CreateDynamicMaterialInstance` "/Game/_Core/FX/M_AfterImage.M_AfterImage"))
  (set `self.MID` _returnvalue)
  (`MaterialInstanceDynamic.SetVectorParameterValue` _mid "Tint" (`self.Tint`))
  (`MaterialInstanceDynamic.SetScalarParameterValue` _mid "Opacity" (`self.StartOpacity`))
  (`PrimitiveComponent.SetMaterial` (`self.PM_Ghost`) 0 (`self.MID`))
  (bind (_direction _alpha) (`Timeline|TL_Fade` :!via `PlayFromStart`)
    (:`Update`
      (`/Engine/EditorBlueprintResources/StandardMacros.IsValid` _mid_2
        (:`Is Valid`
          (`MaterialInstanceDynamic.SetScalarParameterValue` _mid_2 "Opacity" (`KismetMathLibrary.Lerp` (`self.StartOpacity`) (`self.EndOpacity`) _alpha)))))
    (:`Finished`
      (`self.K2_DestroyActor`))))

(event `self.ReceiveBeginPlay`)

(fn `UserConstructionScript`)